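; Floor actor built from sixteen static mesh segments that recycle themselves forward, apparently forming an endless ground.
; When a collision actor stops overlapping a segment, that segment jumps a fixed distance along its local X axis, with identical logic repeated per mesh.
; An additional function, not called in this file, would shift the whole actor forward under the same cast check.
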(event OnComponentEndOverlap(StaticMesh)
  (params (OverlappedComponent :type Primitive%20Component%20Object%20Reference) (OtherActor :type Actor%20Object%20Reference) (OtherComp :type Primitive%20Component%20Object%20Reference) (OtherBodyIndex :type Integer))
  (Utilities|Casting|CastTocollision OtherActor)
  (Transformation|AddLocalOffset OverlappedComponent "700.000000, 0, 0" false false))

(event OnComponentEndOverlap(StaticMesh1)
  (params (OverlappedComponent :type Primitive%20Component%20Object%20Reference) (OtherActor :type Actor%20Object%20Reference) (OtherComp :type Primitive%20Component%20Object%20Reference) (OtherBodyIndex :type Integer))
  (Utilities|Casting|CastTocollision OtherActor)
  (Transformation|AddLocalOffset OverlappedComponent "700.000000, 0, 0" false false))

(event OnComponentEndOverlap(StaticMesh10)
  (params (OverlappedComponent :type Primitive%20Component%20Object%20Reference) (OtherActor :type Actor%20Object%20Reference) (OtherComp :type Primitive%20Component%20Object%20Reference) (OtherBodyIndex :type Integer))
  (Utilities|Casting|CastTocollision OtherActor)
  (Transformation|AddLocalOffset OverlappedComponent "700.000000, 0, 0" false false))

(event OnComponentEndOverlap(StaticMesh11)
  (params (OverlappedComponent :type Primitive%20Component%20Object%20Reference) (OtherActor :type Actor%20Object%20Reference) (OtherComp :type Primitive%20Component%20Object%20Reference) (OtherBodyIndex :type Integer))
  (Utilities|Casting|CastTocollision OtherActor)
  (Transformation|AddLocalOffset OverlappedComponent "700.000000, 0, 0" false false))

(event OnComponentEndOverlap(StaticMesh12)
  (params (OverlappedComponent :type Primitive%20Component%20Object%20Reference) (OtherActor :type Actor%20Object%20Reference) (OtherComp :type Primitive%20Component%20Object%20Reference) (OtherBodyIndex :type Integer))
  (Utilities|Casting|CastTocollision OtherActor)
  (Transformation|AddLocalOffset OverlappedComponent "700.000000, 0, 0" false false))

(event OnComponentEndOverlap(StaticMesh13)
  (params (OverlappedComponent :type Primitive%20Component%20Object%20Reference) (OtherActor :type Actor%20Object%20Reference) (OtherComp :type Primitive%20Component%20Object%20Reference) (OtherBodyIndex :type Integer))
  (Utilities|Casting|CastTocollision OtherActor)
  (Transformation|AddLocalOffset OverlappedComponent "700.000000, 0, 0" false false))

(event OnComponentEndOverlap(StaticMesh14)
  (params (OverlappedComponent :type Primitive%20Component%20Object%20Reference) (OtherActor :type Actor%20Object%20Reference) (OtherComp :type Primitive%20Component%20Object%20Reference) (OtherBodyIndex :type Integer))
  (Utilities|Casting|CastTocollision OtherActor)
  (Transformation|AddLocalOffset OverlappedComponent "700.000000, 0, 0" false false))

(event OnComponentEndOverlap(StaticMesh15)
  (params (OverlappedComponent :type Primitive%20Component%20Object%20Reference) (OtherActor :type Actor%20Object%20Reference) (OtherComp :type Primitive%20Component%20Object%20Reference) (OtherBodyIndex :type Integer))
  (Utilities|Casting|CastTocollision OtherActor)
  (Transformation|AddLocalOffset OverlappedComponent "700.000000, 0, 0" false false))

(event OnComponentEndOverlap(StaticMesh2)
  (params (OverlappedComponent :type Primitive%20Component%20Object%20Reference) (OtherActor :type Actor%20Object%20Reference) (OtherComp :type Primitive%20Component%20Object%20Reference) (OtherBodyIndex :type Integer))
  (Utilities|Casting|CastTocollision OtherActor)
  (Transformation|AddLocalOffset OverlappedComponent "700.000000, 0, 0" false false))

(event OnComponentEndOverlap(StaticMesh3)
  (params (OverlappedComponent :type Primitive%20Component%20Object%20Reference) (OtherActor :type Actor%20Object%20Reference) (OtherComp :type Primitive%20Component%20Object%20Reference) (OtherBodyIndex :type Integer))
  (Utilities|Casting|CastTocollision OtherActor)
  (Transformation|AddLocalOffset OverlappedComponent "700.000000, 0, 0" false false))

(event OnComponentEndOverlap(StaticMesh4)
  (params (OverlappedComponent :type Primitive%20Component%20Object%20Reference) (OtherActor :type Actor%20Object%20Reference) (OtherComp :type Primitive%20Component%20Object%20Reference) (OtherBodyIndex :type Integer))
  (Utilities|Casting|CastTocollision OtherActor)
  (Transformation|AddLocalOffset OverlappedComponent "700.000000, 0, 0" false false))

(event OnComponentEndOverlap(StaticMesh8)
  (params (OverlappedComponent :type Primitive%20Component%20Object%20Reference) (OtherActor :type Actor%20Object%20Reference) (OtherComp :type Primitive%20Component%20Object%20Reference) (OtherBodyIndex :type Integer))
  (Utilities|Casting|CastTocollision OtherActor)
  (Transformation|AddLocalOffset OverlappedComponent "700.000000, 0, 0" false false))

(event OnComponentEndOverlap(StaticMesh6)
  (params (OverlappedComponent :type Primitive%20Component%20Object%20Reference) (OtherActor :type Actor%20Object%20Reference) (OtherComp :type Primitive%20Component%20Object%20Reference) (OtherBodyIndex :type Integer))
  (Utilities|Casting|CastTocollision OtherActor)
  (Transformation|AddLocalOffset OverlappedComponent "700.000000, 0, 0" false false))

(event OnComponentEndOverlap(StaticMesh5)
  (params (OverlappedComponent :type Primitive%20Component%20Object%20Reference) (OtherActor :type Actor%20Object%20Reference) (OtherComp :type Primitive%20Component%20Object%20Reference) (OtherBodyIndex :type Integer))
  (Utilities|Casting|CastTocollision OtherActor)
  (Transformation|AddLocalOffset OverlappedComponent "700.000000, 0, 0" false false))

(event OnComponentEndOverlap(StaticMesh9)
  (params (OverlappedComponent :type Primitive%20Component%20Object%20Reference) (OtherActor :type Actor%20Object%20Reference) (OtherComp :type Primitive%20Component%20Object%20Reference) (OtherBodyIndex :type Integer))
  (Utilities|Casting|CastTocollision OtherActor)
  (Transformation|AddLocalOffset OverlappedComponent "700.000000, 0, 0" false false))

(event OnComponentEndOverlap(StaticMesh7)
  (params (OverlappedComponent :type Primitive%20Component%20Object%20Reference) (OtherActor :type Actor%20Object%20Reference) (OtherComp :type Primitive%20Component%20Object%20Reference) (OtherBodyIndex :type Integer))
  (Utilities|Casting|CastTocollision OtherActor)
  (Transformation|AddLocalOffset OverlappedComponent "700.000000, 0, 0" false false))

(fn ConstructionScript)

(fn NewFunction0
  (params (Object :type Object%20Object%20Reference))
  (Utilities|Casting|CastTocollision Object)
  (Transformation|AddActorLocalOffset "750.000000, 0,0.000000" false false))