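; Obstacle spawner that keeps creating NewBlueprint actors at a fixed X position throughout play.
; BeginPlay spawns one at a default position, then starts a self-calling event that waits a random delay between two variables before each spawn.
; Each later spawn is moved at random into either an upper or a lower height band by setting its transform after creation.
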(event Custom|spawnnext
  (Utilities|FlowControl|Delay (Math|Random|RandomFloatinRange (Variables|Default|GetNewVar_0) (Variables|Default|GetNewVar_1)))
  (bind _returnvalue (CallFunction|Spawn))
  (Utilities|FlowControl|Sequence
    (:then_0
      (if (== (Math|Random|RandomIntegerinRange 1 2) 1)
        (Variables|Default|SetNewVar_2 (Math|Random|RandomFloatinRange 1e+01 15.0))
        (else
          (Variables|Default|SetNewVar_2 (Math|Random|RandomFloatinRange -37.5 -42.5))))
      (Transformation|SetActorTransform _returnvalue (Math|Transform|MakeTransform (Math|Vector|MakeVector 7e+02 0.0 (Variables|Default|GetNewVar_2)) "0, 0, 0" (Math|Vector|MakeVector 1.0 1.0 1.0)))
      (CallFunction|Spawnnext))))

(event EventBeginPlay
  (CallFunction|Spawn)
  (CallFunction|Spawnnext))

(fn ConstructionScript)

(fn Spawn
  (bind _returnvalue (Game|SpawnActorfromClass "/Game/Blueprints/obstacles/NewBlueprint.NewBlueprint_C" (Math|Transform|MakeTransform "700.000000, 0,12.500000" "0, 0, 0" "1,1,1") "Undefined" 0 0))
  (return _returnvalue))